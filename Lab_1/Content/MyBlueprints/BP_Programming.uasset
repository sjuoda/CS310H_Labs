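; BP_Programming is a small Blueprint test that prints the result of an integer helper function when the 0 key is pressed.
; BeginPlay sets two integer variables, which the key event passes to AddNums before printing the return value as a string.
; AddNums contains an addition node marked unused, so the sum is not visibly returned.
; A duplicate print chain sits disconnected, and Tick is empty.
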(event EventBeginPlay
  (Variables|Default|SetMyInt1 5)
  (Variables|Default|SetMyInt2 12))

(event Collision|EventActorBeginOverlap
  (params (OtherActor :type Actor%20Object%20Reference)))

(event EventTick
  (params (DeltaSeconds :type Float%20%28single-precision%29)))

(event Input|KeyboardEvents|0
  (params (Key :type Key%20Structure :default "None"))
  (:Pressed
    (Development|PrintString (Utilities|String|ToString(Integer) (Utilities|AddNums (Variables|Default|GetMyInt1) (Variables|Default|GetMyInt2))))))

(fn ConstructionScript)